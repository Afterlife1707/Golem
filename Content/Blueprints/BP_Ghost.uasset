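; BP_Ghost is a ghost actor that tests the obstacles its capsule overlaps, breaking through path ones and dying on the others.
; For a path obstacle, it spawns an FS_MasterField with explosion effect and sound, then disables the obstacle's collision and sets a short lifespan.
; For any other obstacle, it calls NoPathHit with EjectFromPlayer and destroys itself.
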(event `self.CapsuleComponent.OnComponentBeginOverlap`
  (params (OverlappedComponent :type "PrimitiveComponent Object Reference") (OtherActor :type "Actor Object Reference") (OtherComp :type "PrimitiveComponent Object Reference") (OtherBodyIndex :type Integer) (bFromSweep :type Boolean) (SweepResult :type "HitResult Structure (by ref)"))
  (bind _asbp_obstacle_1 (cast `/Game/Blueprints/Items/BP_Obstacle` OtherActor))
  (if (`/Game/Blueprints/Items/BP_Obstacle.bIsPath` _asbp_obstacle_1)
    (`self.AddForceToGCA` (`self.GetTransform` OtherActor))
    (`self.SetActorEnableCollision` _asbp_obstacle_1 false)
    (`self.SetLifeSpan` _asbp_obstacle_1 2.0)
    (else
      (`/Game/Blueprints/Items/BP_Obstacle.NoPathHit` _asbp_obstacle_1 "/Engine/EditorSounds/GamePreview/EjectFromPlayer.EjectFromPlayer")
      (`self.K2_DestroyActor`))))

(event `AddForceToGCA`
  (params (SpawnTransform :type "Transform Structure"))
  (bind _returnvalue (`|SpawnActorFromClass` "/Engine/EditorResources/FieldNodes/FS_MasterField.FS_MasterField_C" SpawnTransform "AlwaysSpawn" "MultiplyWithRoot" null null))
  (`GameplayStatics.PlaySound2D` "/Game/Assets/Audio/fire.fire" 0.5 1.0 0.0 null null)
  (`GameplayStatics.SpawnEmitterAtLocation` "/Game/StarterContent/Particles/P_Explosion.P_Explosion" (+ (`self.K2_GetActorLocation` _returnvalue) (0.0 0.0 50.0)) (struct) (2.0 2.0 2.0)))

(fn `UserConstructionScript`)