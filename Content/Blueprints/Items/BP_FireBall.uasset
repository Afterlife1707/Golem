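; BP_FireBall is a short-lived fireball projectile that breaks path obstacles and destroys itself after a brief delay.
; Every mesh overlap spawns an explosion emitter, but ghosts are otherwise ignored.
; Path obstacles get a spawned FS_MasterField force, fire sound and instigator camera shake, then lose collision and expire.
; Non-path obstacles receive NoPathHit instead, and obstacle or other non-ghost hits destroy the fireball, with a check against the instigator.
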(event `self.ReceiveBeginPlay`
  (`KismetSystemLibrary.Delay` 1.5)
  (`self.K2_DestroyActor`))

(event `self.StaticMesh.OnComponentBeginOverlap`
  (params (OverlappedComponent :type "PrimitiveComponent Object Reference") (OtherActor :type "Actor Object Reference") (OtherComp :type "PrimitiveComponent Object Reference") (OtherBodyIndex :type Integer) (bFromSweep :type Boolean) (SweepResult :type "HitResult Structure (by ref)"))
  (`GameplayStatics.SpawnEmitterAtLocation` "/Game/StarterContent/Particles/P_Explosion.P_Explosion" (+ (`self.K2_GetActorLocation` OtherActor) (-0.0 0.0 150.0)))
  (cast `/Game/Blueprints/Golem/BP_Ghost` OtherActor
    (:`CastFailed`
      (bind _asbp_obstacle (cast `/Game/Blueprints/Items/BP_Obstacle` OtherActor)
        (:`then`
          (if (`/Game/Blueprints/Items/BP_Obstacle.bIsPath` _asbp_obstacle)
            (`self.AddForceToGCA` (`self.GetTransform` OtherActor))
            (`self.SetActorEnableCollision` _asbp_obstacle false)
            (`self.SetLifeSpan` _asbp_obstacle 0.1)
            (else
              (`/Game/Blueprints/Items/BP_Obstacle.NoPathHit` _asbp_obstacle "/Engine/EditorSounds/GamePreview/EjectFromPlayer.EjectFromPlayer")))
          (`self.K2_DestroyActor` :!label _label))
        (:`CastFailed`
          (if (!= OtherComp (`self.Instigator`))
            (goto _label)))))))

(event `AddForceToGCA`
  (params (SpawnTransform :type "Transform Structure"))
  (bind _returnvalue (`|SpawnActorFromClass` "/Engine/EditorResources/FieldNodes/FS_MasterField.FS_MasterField_C" SpawnTransform "AlwaysSpawn" "MultiplyWithRoot" null null))
  (`GameplayStatics.PlaySound2D` "/Game/Assets/Audio/fire.fire" 0.5 1.0 0.0 null null)
  (`/Game/Blueprints/Golem/BP_MyCharacter.CamShake` (cast `/Game/Blueprints/Golem/BP_MyCharacter` (`self.Instigator`) :!pure true)))

(fn `UserConstructionScript`)