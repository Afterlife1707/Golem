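; Player character for a level-based game that shoots fireballs at the cost of an element bar and dies on touching obstacles.
; GM_BaseLevel configures the HUD and shot cost, while Tick uses a one-second Delay to re-arm shooting.
; A low bar triggers a blood flash; shooting on an empty bar reloads the level by console command.
; It also handles pausing, camera shake, next-level loading and a tutorial ghost hint.
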(event `CamShake`
  ;[1 1 1 1 55] Camera Shake
  (`GameplayStatics.PlayWorldCameraShake` "/Game/Blueprints/Common/BP_CamShake.BP_CamShake_C" (`SceneComponent.K2_GetComponentLocation` (`self.FollowCamera`)) 0.0 10.0 1.0 true))

(event `self.ReceiveTick`
  (params (DeltaSeconds :type "Float (single-precision)"))
  (bind _ui (`self.UI`))
  ;[1 1 1 1 55] Tick
  (if (not (`self.bCanShoot`))
    (`/Game/Blueprints/Widgets/WBP_UI.SetBarEnabled` _ui false)
    (`KismetSystemLibrary.Delay` 1.0)
    (set `self.bCanShoot` true)
    (`/Game/Blueprints/Widgets/WBP_UI.SetBarEnabled` _ui true)
    (`GameplayStatics.PlaySound2D` "/Engine/VREditor/Sounds/UI/Enter_Play.Enter_Play" 0.5 1.0 0.0 null null)))

(event `EnhancedInput|/Game/ThirdPerson/Input/Actions/IA_Pause`
  (params (ActionValue :type Boolean) (ElapsedSeconds :type "Float (double-precision)") (TriggeredSeconds :type "Float (double-precision)") (InputAction :type "InputAction Object Reference" :default "/Game/ThirdPerson/Input/Actions/IA_Pause.IA_Pause"))
  ;[1 1 1 1 55] Pause
  (:`Started`
    (set `self.bIsPaused` (not (`self.bIsPaused`)))
    (if (`self.bIsPaused`)
      (`self.Pause`)
      (else
        (`self.Unpause`)))))

(event `EnhancedInput|/Game/ThirdPerson/Input/Actions/IA_Shoot`
  (params (ActionValue :type Boolean) (ElapsedSeconds :type "Float (double-precision)") (TriggeredSeconds :type "Float (double-precision)") (InputAction :type "InputAction Object Reference" :default "/Game/ThirdPerson/Input/Actions/IA_Shoot.IA_Shoot"))
  ;[1 1 1 1 55] Shoot
  (:`Started`
    (if (`self.bCanShoot`)
      (set `self.bCanShoot` false)
      (`self.SpawnBullet`)
      (`self.Deplete Element Bar` (`/Game/Blueprints/Classes/GM_BaseLevel.HealthToDeplete` (cast `/Game/Blueprints/Classes/GM_BaseLevel` (`GameplayStatics.GetGameMode`) :!pure true))))))

(event `self.CapsuleComponent.OnComponentBeginOverlap`
  (params (OverlappedComponent :type "PrimitiveComponent Object Reference") (OtherActor :type "Actor Object Reference") (OtherComp :type "PrimitiveComponent Object Reference") (OtherBodyIndex :type Integer) (bFromSweep :type Boolean) (SweepResult :type "HitResult Structure (by ref)"))
  ;[1 1 1 1 55] Overlap
  (cast `/Game/Blueprints/Items/BP_Obstacle` OtherActor)
  (`GameplayStatics.PlaySound2D` "/Game/Assets/Audio/hurt.hurt" 0.5 1.0 0.0 null null)
  (`self.Death`)
  (`/Game/Blueprints/Widgets/WBP_UI.FadeOut` (`self.UI`))
  ;;[1 1 1] Ghost Hint Tutorial
  (bind _asgm_tutorial (cast `/Game/Blueprints/Classes/GM_Tutorial` (`GameplayStatics.GetGameMode`)))
  (`/Game/Blueprints/Classes/GM_Tutorial.Show Ghost Hint` _asgm_tutorial))

(event `Pause`
  (bind _returnvalue (`GameplayStatics.GetPlayerController` 0))
  ;[1 1 1 1 55] Pause
  (`self.PauseUI`
    (:`then`
      _)
    (:`else`
      (bind _returnvalue_2 (`|CreateWidget` "/Game/Blueprints/Widgets/WBP_Pause.WBP_Pause_C"))
      (bind _output_get (set `self.PauseUI` _returnvalue_2))))
  (`UserWidget.AddToViewport` (`self.PauseUI`) 0)
  (`WidgetBlueprintLibrary.SetInputMode_UIOnlyEx` _returnvalue _output_get)
  (set `PlayerController.bShowMouseCursor` true _returnvalue)
  (`GameplayStatics.SetGamePaused` true)
  (`/Game/Blueprints/Widgets/WBP_Pause.UpdateButtonsState` _output_get))

(event `Unpause`
  (bind _returnvalue (`GameplayStatics.GetPlayerController` 0))
  ;[1 1 1 1 55] Pause
  (`Widget.RemoveFromParent` (`self.PauseUI`))
  (`WidgetBlueprintLibrary.SetInputMode_GameOnly` _returnvalue)
  (set `PlayerController.bShowMouseCursor` false _returnvalue)
  (`GameplayStatics.SetGamePaused` false))

(event `InitiateFlash`
  ;[1 1 1 1 55] Flash
  (bind _returnvalue (`|CreateWidget` "/Game/Blueprints/Widgets/WBP_Blood.WBP_Blood_C"))
  (`UserWidget.AddToViewport` _returnvalue 0)
  (`/Game/Blueprints/Widgets/WBP_Blood.LoopBlood` _returnvalue))

(event `DelayAndDeath`
  ;[1 1 1 1 55] Death
  (`MovementComponent.StopMovementImmediately` (`self.CharacterMovement`))
  (`self.DisableInput` null)
  (bind _returnvalue (`|CreateWidget` "/Game/Blueprints/Widgets/WBP_Death.WBP_Death_C"))
  (`UserWidget.AddToViewport` _returnvalue 0)
  (`KismetSystemLibrary.Delay` 2.0)
  (`KismetSystemLibrary.ExecuteConsoleCommand` (`KismetStringLibrary.Concat_StrStr` "open Level" (`KismetStringLibrary.Conv_IntToString` (- (`/Game/Blueprints/Classes/GM_BaseLevel.NextLevel` (cast `/Game/Blueprints/Classes/GM_BaseLevel` (`GameplayStatics.GetGameMode`) :!pure true)) 1))) null))

(event `OpenNextLevel`
  ;[1 1 1] Next Level
  (`KismetSystemLibrary.ExecuteConsoleCommand` (`KismetStringLibrary.Concat_StrStr` "open Level" (`KismetStringLibrary.Conv_IntToString` (`/Game/Blueprints/Classes/GM_BaseLevel.NextLevel` (cast `/Game/Blueprints/Classes/GM_BaseLevel` (`GameplayStatics.GetGameMode`) :!pure true)))) null))

(fn `Deplete Element Bar`
  (params (ToDeplete :type "Float (double-precision)"))
  (bind _elementbar (`/Game/Blueprints/Widgets/WBP_UI.ElementBar` (`self.UI`)))
  (bind _percent (`ProgressBar.Percent` _elementbar))
  (if (<= _percent 0.0)
    (`self.DelayAndDeath`)
    (else
      (`KismetSystemLibrary.PrintString` (`KismetStringLibrary.Conv_DoubleToString` _percent))
      (set `ProgressBar.Percent` (- _percent ToDeplete) _elementbar)
      (if (<= _percent 0.15)
        (`self.InitiateFlash`)))))

(fn `InitUI`
  (bind _asgm_base_level (cast `/Game/Blueprints/Classes/GM_BaseLevel` (`GameplayStatics.GetGameMode`) :!pure true))
  (bind _returnvalue (`|CreateWidget` "/Game/Blueprints/Widgets/WBP_UI.WBP_UI_C" null (`/Game/Blueprints/Classes/GM_BaseLevel.BarColor` _asgm_base_level) (`/Game/Blueprints/Classes/GM_BaseLevel.TimeForRound` _asgm_base_level) (`/Game/Blueprints/Classes/GM_BaseLevel.IntroText` _asgm_base_level)))
  (bind _output_get (set `self.UI` _returnvalue))
  (`UserWidget.AddToViewport` _output_get 0)
  (`/Game/Blueprints/Widgets/WBP_UI.FadeOut` _output_get)
  (`/Game/Blueprints/Widgets/WBP_UI.StartTimer` _returnvalue))

(fn `SetInput`
  (params (Enable :type Boolean))
  (if Enable
    (`self.EnableInput` null)
    (else
      (`self.DisableInput` null))))

(fn `SpawnBullet`
  (`GameplayStatics.PlaySound2D` "/Game/Assets/Audio/fireball.fireball" 0.5 1.0 0.0 null null)
  (`MovementComponent.StopMovementImmediately` (`self.CharacterMovement`))
  (`self.DisableInput` null)
  (`|SpawnActorFromClass` "/Game/Blueprints/Items/BP_FireBall.BP_FireBall_C" (`SceneComponent.K2_GetComponentToWorld` (`self.LaunchPos`)) "AdjustIfPossibleButAlwaysSpawn" "MultiplyWithRoot" null self)
  (`self.EnableInput` null))

(fn `UserConstructionScript`)